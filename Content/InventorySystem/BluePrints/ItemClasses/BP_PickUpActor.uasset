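; BP_PickUpActor is a world pickup that adds a configured item and amount to the player's inventory.
; When a BP_2DSideScrollerCharacter overlaps its Sphere, it calls AddItem on that character's InventoryRef if the reference is valid.
; On success, any leftover becomes the pickup's new Amount, and the actor destroys itself once nothing remains.
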(event `self.Sphere.OnComponentBeginOverlap`
  (params (OverlappedComponent :type "PrimitiveComponent Object Reference") (OtherActor :type "Actor Object Reference") (OtherComp :type "PrimitiveComponent Object Reference") (OtherBodyIndex :type Integer) (bFromSweep :type Boolean) (SweepResult :type "HitResult Structure (by ref)"))
  (bind _asbp_2dside_scroller_character (cast `/Game/2DSideScrollerCPP/Blueprints/BP_2DSideScrollerCharacter` OtherActor))
  (bind _inventoryref (`/Game/2DSideScrollerCPP/Blueprints/BP_2DSideScrollerCharacter.InventoryRef` _asbp_2dside_scroller_character))
  (`/Engine/EditorBlueprintResources/StandardMacros.IsValid` _inventoryref
    (:`Is Valid`
      (bind (_succes_ _rest) (`/Game/InventorySystem/BluePrints/BP_Inventory.AddItem` _inventoryref (`self.ItemToAdd`) (`self.Amount`)))
      (if _succes_
        (if (> _rest 0)
          (set `self.Amount` _rest)
          (else
            (`self.K2_DestroyActor`)))))))

(fn `UserConstructionScript`)